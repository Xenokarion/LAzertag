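; BP_Controll is a controller Blueprint that drives bomb-plant zone visuals, labelled A or B, and an explosion.
; Tick polls the PlantedZone1, PlantedZone2 and Explosion booleans, each through a DoOnce that resets when the flag clears.
; A plant flag teleports the shared zone actor to that site, plays its sequence and sets the 3D letter.
; Explosion reverses the zone sequence and plays the explosion sequence.
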(event EventBeginPlay)

(event Collision|EventActorBeginOverlap
  (params (OtherActor :type Actor%20Object%20Reference)))

(event EventTick
  (params (DeltaSeconds :type Float%20%28single-precision%29))
  (bind _zonetext3d (Variables|Default|GetZoneText3d))
  (bind _text3dcomponent (Variables|/Script/Text3D.Text3DActor|GetText3DComponent _zonetext3d))
  (Utilities|FlowControl|Sequence
    (:then_1
      (if (Variables|Default|GetbPlantedZone1)
        (Utilities|FlowControl|DoOnce false :!label _label
          (:Completed
            (Transformation|SetActorLocation (Variables|Default|GetPlantedZone) "1650.000000,200.000000,2140.000000" false true)
            (Sequencer|Player|Play (Variables|/Script/LevelSequence.LevelSequenceActor|GetSequencePlayer (Variables|Default|GetPlantedZoneSeq)) :!class /Script/MovieScene.MovieSceneSequencePlayer)
            (Variables|/Script/Text3D.Text3DComponent|SetText _text3dcomponent "A")))
        (else
          (goto _label Reset))))
    (:then_2
      (if (Variables|Default|GetbPlantedZone2)
        (Utilities|FlowControl|DoOnce false :!label _label_2
          (:Completed
            (Transformation|SetActorLocation (Variables|Default|GetPlantedZone) "3484.000000,200.000000,2140.000000" false true)
            (Sequencer|Player|Play (Variables|/Script/LevelSequence.LevelSequenceActor|GetSequencePlayer (Variables|Default|GetPlantedZoneSeq)) :!class /Script/MovieScene.MovieSceneSequencePlayer)
            (Variables|/Script/Text3D.Text3DComponent|SetText _text3dcomponent "B")))
        (else
          (goto _label_2 Reset))))
    (:then_3
      (if (Variables|Default|GetbExplosion)
        (Utilities|FlowControl|DoOnce false :!label _label_3
          (:Completed
            (Class|MovieSceneSequencePlayer|PlayReverse (Variables|/Script/LevelSequence.LevelSequenceActor|GetSequencePlayer (Variables|Default|GetPlantedZoneSeq)))
            (Sequencer|Player|Play (Variables|/Script/LevelSequence.LevelSequenceActor|GetSequencePlayer (Variables|Default|GetExplosionSeq)) :!class /Script/MovieScene.MovieSceneSequencePlayer)))
        (else
          (goto _label_3 Reset))))))

(fn ConstructionScript)