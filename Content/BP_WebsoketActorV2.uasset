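; Actor that shows live markers for two teams of seven athletes, driven by JSON from a WebSocket feed opened on BeginPlay.
; Each message updates label child actors' health, number, nickname, id and visibility from isPlaying, storing new positions only when they move beyond a jitter threshold.
; A looping timer eases each marker toward its stored position with camera-relative pitch and yaw, and stops when the socket closes.
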(event Custom|WebSocketConected
  (params (b :type Boolean))
  (Development|PrintString (Utilities|String|Append "Conected: " (Utilities|String|ToString(Boolean) b)) true true "(R=0.957051,G=0.989953,B=1.000000,A=1.000000)" 2e+01))

(event Custom|WebSocketConectedError
  (params (error :type String))
  (Development|PrintString (Utilities|String|Append "Conected Error: " error) true true "(R=1.000000,G=0.000000,B=0.064424,A=1.000000)" 2e+01))

(event Custom|WebSocketClosed
  (params (StatusCode :type Integer) (Reason :type String) (bWasClean :type Boolean))
  (Development|PrintString (Utilities|String|Append "Conected close: " (Utilities|String|ToString(Integer) StatusCode)) true true "(R=0.000000,G=1.000000,B=0.974743,A=1.000000)" 3e+02)
  (Utilities|Time|ClearandInvalidateTimerbyHandle (Variables|Default|GetMoveTimer)))

(event Custom|WebSocketTextMessage
  (params (message :type String))
  (for (_array_element _array_index) (Class|BlueprintJsonLibrary|ToArray(JsonValue) (Class|BlueprintJsonLibrary|ToJsonValue(JsonObject) (Class|BlueprintJsonLibrary|ToJsonObject(String) message) "teams"))
    (for (_array_element_2 _array_index_2) (Class|BlueprintJsonLibrary|ToArray(JsonValue) (Class|BlueprintJsonLibrary|ToJsonValue(JsonObject) (Class|BlueprintJsonLibrary|ToObject(JsonValue) _array_element) "athletes"))
      (Utilities|LengthChangeCoordVector (Utilities|Select :Index _array_index :Option%200 (Utilities|Select :Index _array_index_2 :Option%200 (Variables|Default|GetCoordPlayer1_1) :Option%201 (Variables|Default|GetCoordPlayer1_2) :Option%202 (Variables|Default|GetCoordPlayer1_3) :Option%203 (Variables|Default|GetCoordPlayer1_4) :Option%204 (Variables|Default|GetCoordPlayer1_5) :Option%205 (Variables|Default|GetCoordPlayer1_6) :Option%206 (Variables|Default|GetCoordPlayer1_7)) :Option%201 (Utilities|Select :Index _array_index_2 :Option%200 (Variables|Default|GetCoordPlayer2_1) :Option%201 (Variables|Default|GetCoordPlayer2_2) :Option%202 (Variables|Default|GetCoordPlayer2_3) :Option%203 (Variables|Default|GetCoordPlayer2_4) :Option%204 (Variables|Default|GetCoordPlayer2_5) :Option%205 (Variables|Default|GetCoordPlayer2_6) :Option%206 (Variables|Default|GetCoordPlayer2_7))) (Math|Vector|MakeVector (Class|BlueprintJsonLibrary|ToFloat(JsonValue) (Class|BlueprintJsonLibrary|ToJsonValue(JsonObject) (Class|BlueprintJsonLibrary|ToObject(JsonValue) (Class|BlueprintJsonLibrary|ToJsonValue(JsonObject) (Class|BlueprintJsonLibrary|ToObject(JsonValue) _array_element_2) "position")) "x")) (Class|BlueprintJsonLibrary|ToFloat(JsonValue) (Class|BlueprintJsonLibrary|ToJsonValue(JsonObject) (Class|BlueprintJsonLibrary|ToObject(JsonValue) (Class|BlueprintJsonLibrary|ToJsonValue(JsonObject) (Class|BlueprintJsonLibrary|ToObject(JsonValue) _array_element_2) "position")) "y")) (Variables|Default|GetZPoz))
        (:true
          (switch int _array_index
            (:0
              (switch int _array_index_2
                (:0
                  (Variables|Default|SetCoordPlayer1_1 (Math|Vector|MakeVector (Class|BlueprintJsonLibrary|ToFloat(JsonValue) (Class|BlueprintJsonLibrary|ToJsonValue(JsonObject) (Class|BlueprintJsonLibrary|ToObject(JsonValue) (Class|BlueprintJsonLibrary|ToJsonValue(JsonObject) (Class|BlueprintJsonLibrary|ToObject(JsonValue) _array_element_2) "position")) "x")) (Class|BlueprintJsonLibrary|ToFloat(JsonValue) (Class|BlueprintJsonLibrary|ToJsonValue(JsonObject) (Class|BlueprintJsonLibrary|ToObject(JsonValue) (Class|BlueprintJsonLibrary|ToJsonValue(JsonObject) (Class|BlueprintJsonLibrary|ToObject(JsonValue) _array_element_2) "position")) "y")) (Variables|Default|GetZPoz))))
                (:1
                  (Variables|Default|SetCoordPlayer1_2 (Math|Vector|MakeVector (Class|BlueprintJsonLibrary|ToFloat(JsonValue) (Class|BlueprintJsonLibrary|ToJsonValue(JsonObject) (Class|BlueprintJsonLibrary|ToObject(JsonValue) (Class|BlueprintJsonLibrary|ToJsonValue(JsonObject) (Class|BlueprintJsonLibrary|ToObject(JsonValue) _array_element_2) "position")) "x")) (Class|BlueprintJsonLibrary|ToFloat(JsonValue) (Class|BlueprintJsonLibrary|ToJsonValue(JsonObject) (Class|BlueprintJsonLibrary|ToObject(JsonValue) (Class|BlueprintJsonLibrary|ToJsonValue(JsonObject) (Class|BlueprintJsonLibrary|ToObject(JsonValue) _array_element_2) "position")) "y")) (Variables|Default|GetZPoz))))
                (:2
                  (Variables|Default|SetCoordPlayer1_3 (Math|Vector|MakeVector (Class|BlueprintJsonLibrary|ToFloat(JsonValue) (Class|BlueprintJsonLibrary|ToJsonValue(JsonObject) (Class|BlueprintJsonLibrary|ToObject(JsonValue) (Class|BlueprintJsonLibrary|ToJsonValue(JsonObject) (Class|BlueprintJsonLibrary|ToObject(JsonValue) _array_element_2) "position")) "x")) (Class|BlueprintJsonLibrary|ToFloat(JsonValue) (Class|BlueprintJsonLibrary|ToJsonValue(JsonObject) (Class|BlueprintJsonLibrary|ToObject(JsonValue) (Class|BlueprintJsonLibrary|ToJsonValue(JsonObject) (Class|BlueprintJsonLibrary|ToObject(JsonValue) _array_element_2) "position")) "y")) (Variables|Default|GetZPoz))))
                (:3
                  (Variables|Default|SetCoordPlayer1_4 (Math|Vector|MakeVector (Class|BlueprintJsonLibrary|ToFloat(JsonValue) (Class|BlueprintJsonLibrary|ToJsonValue(JsonObject) (Class|BlueprintJsonLibrary|ToObject(JsonValue) (Class|BlueprintJsonLibrary|ToJsonValue(JsonObject) (Class|BlueprintJsonLibrary|ToObject(JsonValue) _array_element_2) "position")) "x")) (Class|BlueprintJsonLibrary|ToFloat(JsonValue) (Class|BlueprintJsonLibrary|ToJsonValue(JsonObject) (Class|BlueprintJsonLibrary|ToObject(JsonValue) (Class|BlueprintJsonLibrary|ToJsonValue(JsonObject) (Class|BlueprintJsonLibrary|ToObject(JsonValue) _array_element_2) "position")) "y")) (Variables|Default|GetZPoz))))
                (:4
                  (Variables|Default|SetCoordPlayer1_5 (Math|Vector|MakeVector (Class|BlueprintJsonLibrary|ToFloat(JsonValue) (Class|BlueprintJsonLibrary|ToJsonValue(JsonObject) (Class|BlueprintJsonLibrary|ToObject(JsonValue) (Class|BlueprintJsonLibrary|ToJsonValue(JsonObject) (Class|BlueprintJsonLibrary|ToObject(JsonValue) _array_element_2) "position")) "x")) (Class|BlueprintJsonLibrary|ToFloat(JsonValue) (Class|BlueprintJsonLibrary|ToJsonValue(JsonObject) (Class|BlueprintJsonLibrary|ToObject(JsonValue) (Class|BlueprintJsonLibrary|ToJsonValue(JsonObject) (Class|BlueprintJsonLibrary|ToObject(JsonValue) _array_element_2) "position")) "y")) (Variables|Default|GetZPoz))))
                (:5
                  (Variables|Default|SetCoordPlayer1_6 (Math|Vector|MakeVector (Class|BlueprintJsonLibrary|ToFloat(JsonValue) (Class|BlueprintJsonLibrary|ToJsonValue(JsonObject) (Class|BlueprintJsonLibrary|ToObject(JsonValue) (Class|BlueprintJsonLibrary|ToJsonValue(JsonObject) (Class|BlueprintJsonLibrary|ToObject(JsonValue) _array_element_2) "position")) "x")) (Class|BlueprintJsonLibrary|ToFloat(JsonValue) (Class|BlueprintJsonLibrary|ToJsonValue(JsonObject) (Class|BlueprintJsonLibrary|ToObject(JsonValue) (Class|BlueprintJsonLibrary|ToJsonValue(JsonObject) (Class|BlueprintJsonLibrary|ToObject(JsonValue) _array_element_2) "position")) "y")) (Variables|Default|GetZPoz))))
                (:6
                  (Variables|Default|SetCoordPlayer1_7 (Math|Vector|MakeVector (Class|BlueprintJsonLibrary|ToFloat(JsonValue) (Class|BlueprintJsonLibrary|ToJsonValue(JsonObject) (Class|BlueprintJsonLibrary|ToObject(JsonValue) (Class|BlueprintJsonLibrary|ToJsonValue(JsonObject) (Class|BlueprintJsonLibrary|ToObject(JsonValue) _array_element_2) "position")) "x")) (Class|BlueprintJsonLibrary|ToFloat(JsonValue) (Class|BlueprintJsonLibrary|ToJsonValue(JsonObject) (Class|BlueprintJsonLibrary|ToObject(JsonValue) (Class|BlueprintJsonLibrary|ToJsonValue(JsonObject) (Class|BlueprintJsonLibrary|ToObject(JsonValue) _array_element_2) "position")) "y")) (Variables|Default|GetZPoz))))))
            (:1
              (switch int _array_index_2
                (:0
                  (Variables|Default|SetCoordPlayer2_1 (Math|Vector|MakeVector (Class|BlueprintJsonLibrary|ToFloat(JsonValue) (Class|BlueprintJsonLibrary|ToJsonValue(JsonObject) (Class|BlueprintJsonLibrary|ToObject(JsonValue) (Class|BlueprintJsonLibrary|ToJsonValue(JsonObject) (Class|BlueprintJsonLibrary|ToObject(JsonValue) _array_element_2) "position")) "x")) (Class|BlueprintJsonLibrary|ToFloat(JsonValue) (Class|BlueprintJsonLibrary|ToJsonValue(JsonObject) (Class|BlueprintJsonLibrary|ToObject(JsonValue) (Class|BlueprintJsonLibrary|ToJsonValue(JsonObject) (Class|BlueprintJsonLibrary|ToObject(JsonValue) _array_element_2) "position")) "y")) (Variables|Default|GetZPoz))))
                (:1
                  (Variables|Default|SetCoordPlayer2_2 (Math|Vector|MakeVector (Class|BlueprintJsonLibrary|ToFloat(JsonValue) (Class|BlueprintJsonLibrary|ToJsonValue(JsonObject) (Class|BlueprintJsonLibrary|ToObject(JsonValue) (Class|BlueprintJsonLibrary|ToJsonValue(JsonObject) (Class|BlueprintJsonLibrary|ToObject(JsonValue) _array_element_2) "position")) "x")) (Class|BlueprintJsonLibrary|ToFloat(JsonValue) (Class|BlueprintJsonLibrary|ToJsonValue(JsonObject) (Class|BlueprintJsonLibrary|ToObject(JsonValue) (Class|BlueprintJsonLibrary|ToJsonValue(JsonObject) (Class|BlueprintJsonLibrary|ToObject(JsonValue) _array_element_2) "position")) "y")) (Variables|Default|GetZPoz))))
                (:2
                  (Variables|Default|SetCoordPlayer2_3 (Math|Vector|MakeVector (Class|BlueprintJsonLibrary|ToFloat(JsonValue) (Class|BlueprintJsonLibrary|ToJsonValue(JsonObject) (Class|BlueprintJsonLibrary|ToObject(JsonValue) (Class|BlueprintJsonLibrary|ToJsonValue(JsonObject) (Class|BlueprintJsonLibrary|ToObject(JsonValue) _array_element_2) "position")) "x")) (Class|BlueprintJsonLibrary|ToFloat(JsonValue) (Class|BlueprintJsonLibrary|ToJsonValue(JsonObject) (Class|BlueprintJsonLibrary|ToObject(JsonValue) (Class|BlueprintJsonLibrary|ToJsonValue(JsonObject) (Class|BlueprintJsonLibrary|ToObject(JsonValue) _array_element_2) "position")) "y")) (Variables|Default|GetZPoz))))
                (:3
                  (Variables|Default|SetCoordPlayer2_4 (Math|Vector|MakeVector (Class|BlueprintJsonLibrary|ToFloat(JsonValue) (Class|BlueprintJsonLibrary|ToJsonValue(JsonObject) (Class|BlueprintJsonLibrary|ToObject(JsonValue) (Class|BlueprintJsonLibrary|ToJsonValue(JsonObject) (Class|BlueprintJsonLibrary|ToObject(JsonValue) _array_element_2) "position")) "x")) (Class|BlueprintJsonLibrary|ToFloat(JsonValue) (Class|BlueprintJsonLibrary|ToJsonValue(JsonObject) (Class|BlueprintJsonLibrary|ToObject(JsonValue) (Class|BlueprintJsonLibrary|ToJsonValue(JsonObject) (Class|BlueprintJsonLibrary|ToObject(JsonValue) _array_element_2) "position")) "y")) (Variables|Default|GetZPoz))))
                (:4
                  (Variables|Default|SetCoordPlayer2_5 (Math|Vector|MakeVector (Class|BlueprintJsonLibrary|ToFloat(JsonValue) (Class|BlueprintJsonLibrary|ToJsonValue(JsonObject) (Class|BlueprintJsonLibrary|ToObject(JsonValue) (Class|BlueprintJsonLibrary|ToJsonValue(JsonObject) (Class|BlueprintJsonLibrary|ToObject(JsonValue) _array_element_2) "position")) "x")) (Class|BlueprintJsonLibrary|ToFloat(JsonValue) (Class|BlueprintJsonLibrary|ToJsonValue(JsonObject) (Class|BlueprintJsonLibrary|ToObject(JsonValue) (Class|BlueprintJsonLibrary|ToJsonValue(JsonObject) (Class|BlueprintJsonLibrary|ToObject(JsonValue) _array_element_2) "position")) "y")) (Variables|Default|GetZPoz))))
                (:5
                  (Variables|Default|SetCoordPlayer2_6 (Math|Vector|MakeVector (Class|BlueprintJsonLibrary|ToFloat(JsonValue) (Class|BlueprintJsonLibrary|ToJsonValue(JsonObject) (Class|BlueprintJsonLibrary|ToObject(JsonValue) (Class|BlueprintJsonLibrary|ToJsonValue(JsonObject) (Class|BlueprintJsonLibrary|ToObject(JsonValue) _array_element_2) "position")) "x")) (Class|BlueprintJsonLibrary|ToFloat(JsonValue) (Class|BlueprintJsonLibrary|ToJsonValue(JsonObject) (Class|BlueprintJsonLibrary|ToObject(JsonValue) (Class|BlueprintJsonLibrary|ToJsonValue(JsonObject) (Class|BlueprintJsonLibrary|ToObject(JsonValue) _array_element_2) "position")) "y")) (Variables|Default|GetZPoz))))
                (:6
                  (Variables|Default|SetCoordPlayer2_7 (Math|Vector|MakeVector (Class|BlueprintJsonLibrary|ToFloat(JsonValue) (Class|BlueprintJsonLibrary|ToJsonValue(JsonObject) (Class|BlueprintJsonLibrary|ToObject(JsonValue) (Class|BlueprintJsonLibrary|ToJsonValue(JsonObject) (Class|BlueprintJsonLibrary|ToObject(JsonValue) _array_element_2) "position")) "x")) (Class|BlueprintJsonLibrary|ToFloat(JsonValue) (Class|BlueprintJsonLibrary|ToJsonValue(JsonObject) (Class|BlueprintJsonLibrary|ToObject(JsonValue) (Class|BlueprintJsonLibrary|ToJsonValue(JsonObject) (Class|BlueprintJsonLibrary|ToObject(JsonValue) _array_element_2) "position")) "y")) (Variables|Default|GetZPoz))))))))
        (:false
          _))
      (if (!= (Variables|/Script/Engine.Actor|GetbHidden (Variables|/Script/Engine.ChildActorComponent|GetChildActor (Utilities|Select :Index _array_index :Option%200 (Utilities|Select :Index _array_index_2 :Option%200 (Variables|Default|GetPlayer1_1) :Option%201 (Variables|Default|GetPlayer1_2) :Option%202 (Variables|Default|GetPlayer1_3) :Option%203 (Variables|Default|GetPlayer1_4) :Option%204 (Variables|Default|GetPlayer1_5) :Option%205 (Variables|Default|GetPlayer1_6) :Option%206 (Variables|Default|GetPlayer1_7)) :Option%201 (Utilities|Select :Index _array_index_2 :Option%200 (Variables|Default|GetPlayer2_1) :Option%201 (Variables|Default|GetPlayer2_2) :Option%202 (Variables|Default|GetPlayer2_3) :Option%203 (Variables|Default|GetPlayer2_4) :Option%204 (Variables|Default|GetPlayer2_5) :Option%205 (Variables|Default|GetPlayer2_6) :Option%206 (Variables|Default|GetPlayer2_7))))) (Class|BlueprintJsonLibrary|ToBoolean(JsonValue) (Class|BlueprintJsonLibrary|ToJsonValue(JsonObject) (Class|BlueprintJsonLibrary|ToObject(JsonValue) _array_element_2) "isPlaying")))
        (bind _asbp_lable_actor (Utilities|Casting|CastToBP_LableActor (Variables|/Script/Engine.ChildActorComponent|GetChildActor (Utilities|Select :Index _array_index :Option%200 (Utilities|Select :Index _array_index_2 :Option%200 (Variables|Default|GetPlayer1_1) :Option%201 (Variables|Default|GetPlayer1_2) :Option%202 (Variables|Default|GetPlayer1_3) :Option%203 (Variables|Default|GetPlayer1_4) :Option%204 (Variables|Default|GetPlayer1_5) :Option%205 (Variables|Default|GetPlayer1_6) :Option%206 (Variables|Default|GetPlayer1_7)) :Option%201 (Utilities|Select :Index _array_index_2 :Option%200 (Variables|Default|GetPlayer2_1) :Option%201 (Variables|Default|GetPlayer2_2) :Option%202 (Variables|Default|GetPlayer2_3) :Option%203 (Variables|Default|GetPlayer2_4) :Option%204 (Variables|Default|GetPlayer2_5) :Option%205 (Variables|Default|GetPlayer2_6) :Option%206 (Variables|Default|GetPlayer2_7)))) :!label _label))
        (Default|UpdateInform _asbp_lable_actor (Class|BlueprintJsonLibrary|ToFloat(JsonValue) (Class|BlueprintJsonLibrary|ToJsonValue(JsonObject) (Class|BlueprintJsonLibrary|ToObject(JsonValue) _array_element_2) "health")) (Class|BlueprintJsonLibrary|ToString(JsonValue) (Class|BlueprintJsonLibrary|ToJsonValue(JsonObject) (Class|BlueprintJsonLibrary|ToObject(JsonValue) _array_element_2) "number")) (Class|BlueprintJsonLibrary|ToString(JsonValue) (Class|BlueprintJsonLibrary|ToJsonValue(JsonObject) (Class|BlueprintJsonLibrary|ToObject(JsonValue) _array_element_2) "nickname")) (Class|BlueprintJsonLibrary|ToInteger(JsonValue) (Class|BlueprintJsonLibrary|ToJsonValue(JsonObject) (Class|BlueprintJsonLibrary|ToObject(JsonValue) _array_element_2) "id")))
        (elif (Variables|/Script/Engine.Actor|GetbHidden (Variables|/Script/Engine.ChildActorComponent|GetChildActor (Utilities|Select :Index _array_index :Option%200 (Utilities|Select :Index _array_index_2 :Option%200 (Variables|Default|GetPlayer1_1) :Option%201 (Variables|Default|GetPlayer1_2) :Option%202 (Variables|Default|GetPlayer1_3) :Option%203 (Variables|Default|GetPlayer1_4) :Option%204 (Variables|Default|GetPlayer1_5) :Option%205 (Variables|Default|GetPlayer1_6) :Option%206 (Variables|Default|GetPlayer1_7)) :Option%201 (Utilities|Select :Index _array_index_2 :Option%200 (Variables|Default|GetPlayer2_1) :Option%201 (Variables|Default|GetPlayer2_2) :Option%202 (Variables|Default|GetPlayer2_3) :Option%203 (Variables|Default|GetPlayer2_4) :Option%204 (Variables|Default|GetPlayer2_5) :Option%205 (Variables|Default|GetPlayer2_6) :Option%206 (Variables|Default|GetPlayer2_7)))))
          (Rendering|SetActorHiddenInGame false)
          (goto _label)
          (else
            (Rendering|SetActorHiddenInGame (Variables|/Script/Engine.ChildActorComponent|GetChildActor (Utilities|Select :Index _array_index :Option%200 (Utilities|Select :Index _array_index_2 :Option%200 (Variables|Default|GetPlayer1_1) :Option%201 (Variables|Default|GetPlayer1_2) :Option%202 (Variables|Default|GetPlayer1_3) :Option%203 (Variables|Default|GetPlayer1_4) :Option%204 (Variables|Default|GetPlayer1_5) :Option%205 (Variables|Default|GetPlayer1_6) :Option%206 (Variables|Default|GetPlayer1_7)) :Option%201 (Utilities|Select :Index _array_index_2 :Option%200 (Variables|Default|GetPlayer2_1) :Option%201 (Variables|Default|GetPlayer2_2) :Option%202 (Variables|Default|GetPlayer2_3) :Option%203 (Variables|Default|GetPlayer2_4) :Option%204 (Variables|Default|GetPlayer2_5) :Option%205 (Variables|Default|GetPlayer2_6) :Option%206 (Variables|Default|GetPlayer2_7)))) true)))))))

(event Custom|WebSocketRawMessage
  (params (data :type Array%20of%20Bytes) (Size :type Integer) (BytesRemaining :type Integer)))

(event Custom|1
  (bind _asbp_lable_actor (Utilities|Casting|CastToBP_LableActor (Variables|/Script/Engine.ChildActorComponent|GetChildActor (Variables|Default|GetPlayer2_4))))
  (Default|CustomEvent _asbp_lable_actor))

(event Custom|2
  (bind _asbp_lable_actor (Utilities|Casting|CastToBP_LableActor (Variables|/Script/Engine.ChildActorComponent|GetChildActor (Variables|Default|GetPlayer1_6))))
  (Default|CustomEvent _asbp_lable_actor))

(event Custom|MoveMark
  (bind _player2_4 (Variables|Default|GetPlayer2_4))
  (bind _player2_5 (Variables|Default|GetPlayer2_5))
  (bind _player2_6 (Variables|Default|GetPlayer2_6))
  (bind _player2_7 (Variables|Default|GetPlayer2_7))
  (bind _player1_1 (Variables|Default|GetPlayer1_1))
  (bind _player1_2 (Variables|Default|GetPlayer1_2))
  (bind _player1_3 (Variables|Default|GetPlayer1_3))
  (bind _player1_4 (Variables|Default|GetPlayer1_4))
  (bind _player1_5 (Variables|Default|GetPlayer1_5))
  (bind _player1_6 (Variables|Default|GetPlayer1_6))
  (bind _player1_7 (Variables|Default|GetPlayer1_7))
  (bind _player2_1 (Variables|Default|GetPlayer2_1))
  (bind _player2_2 (Variables|Default|GetPlayer2_2))
  (bind _player2_3 (Variables|Default|GetPlayer2_3))
  (bind (_returnvalue_yaw _return_value_y__pitch_) (Utilities|RelotivRotationtoCameraMacros _player2_5))
  (bind (_returnvalue_yaw_2 _return_value_y__pitch__2) (Utilities|RelotivRotationtoCameraMacros _player2_6))
  (bind (_returnvalue_yaw_3 _return_value_y__pitch__3) (Utilities|RelotivRotationtoCameraMacros _player1_1))
  (bind (_returnvalue_yaw_4 _return_value_y__pitch__4) (Utilities|RelotivRotationtoCameraMacros _player1_2))
  (bind (_returnvalue_yaw_5 _return_value_y__pitch__5) (Utilities|RelotivRotationtoCameraMacros _player1_3))
  (bind (_returnvalue_yaw_6 _return_value_y__pitch__6) (Utilities|RelotivRotationtoCameraMacros _player1_4))
  (bind (_returnvalue_yaw_7 _return_value_y__pitch__7) (Utilities|RelotivRotationtoCameraMacros _player1_5))
  (bind (_returnvalue_yaw_8 _return_value_y__pitch__8) (Utilities|RelotivRotationtoCameraMacros _player1_6))
  (bind (_returnvalue_yaw_9 _return_value_y__pitch__9) (Utilities|RelotivRotationtoCameraMacros _player1_7))
  (bind (_returnvalue_yaw_10 _return_value_y__pitch__10) (Utilities|RelotivRotationtoCameraMacros _player2_7))
  (bind (_returnvalue_yaw_11 _return_value_y__pitch__11) (Utilities|RelotivRotationtoCameraMacros _player2_1))
  (bind (_returnvalue_yaw_12 _return_value_y__pitch__12) (Utilities|RelotivRotationtoCameraMacros _player2_2))
  (bind (_returnvalue_yaw_13 _return_value_y__pitch__13) (Utilities|RelotivRotationtoCameraMacros _player2_3))
  (bind (_returnvalue_yaw_14 _return_value_y__pitch__14) (Utilities|RelotivRotationtoCameraMacros _player2_4))
  (Utilities|FlowControl|Sequence
    (:then_0
      (Components|MoveComponentTo _player1_1 (Variables|Default|GetCoordPlayer1_1) (Math|Rotator|MakeRotator 0.0 _return_value_y__pitch__3 _returnvalue_yaw_3) false false (Variables|Default|GetOver%20Time) false))
    (:then_1
      (Components|MoveComponentTo _player1_2 (Variables|Default|GetCoordPlayer1_2) (Math|Rotator|MakeRotator 0.0 _return_value_y__pitch__4 _returnvalue_yaw_4) false false (Variables|Default|GetOver%20Time) false))
    (:then_2
      (Components|MoveComponentTo _player1_3 (Variables|Default|GetCoordPlayer1_3) (Math|Rotator|MakeRotator 0.0 _return_value_y__pitch__5 _returnvalue_yaw_5) false false (Variables|Default|GetOver%20Time) false))
    (:then_3
      (Components|MoveComponentTo _player1_4 (Variables|Default|GetCoordPlayer1_4) (Math|Rotator|MakeRotator 0.0 _return_value_y__pitch__6 _returnvalue_yaw_6) false false (Variables|Default|GetOver%20Time) false))
    (:then_4
      (Components|MoveComponentTo _player1_5 (Variables|Default|GetCoordPlayer1_5) (Math|Rotator|MakeRotator 0.0 _return_value_y__pitch__7 _returnvalue_yaw_7) false false (Variables|Default|GetOver%20Time) false))
    (:then_5
      (Components|MoveComponentTo _player1_6 (Variables|Default|GetCoordPlayer1_6) (Math|Rotator|MakeRotator 0.0 _return_value_y__pitch__8 _returnvalue_yaw_8) false false (Variables|Default|GetOver%20Time) false))
    (:then_6
      (Components|MoveComponentTo _player1_7 (Variables|Default|GetCoordPlayer1_7) (Math|Rotator|MakeRotator 0.0 _return_value_y__pitch__9 _returnvalue_yaw_9) false false (Variables|Default|GetOver%20Time) false))
    (:then_7
      (Components|MoveComponentTo _player2_1 (Variables|Default|GetCoordPlayer2_1) (Math|Rotator|MakeRotator 0.0 _return_value_y__pitch__11 _returnvalue_yaw_11) false false (Variables|Default|GetOver%20Time) false))
    (:then_8
      (Components|MoveComponentTo _player2_2 (Variables|Default|GetCoordPlayer2_2) (Math|Rotator|MakeRotator 0.0 _return_value_y__pitch__12 _returnvalue_yaw_12) false false (Variables|Default|GetOver%20Time) false))
    (:then_9
      (Components|MoveComponentTo _player2_3 (Variables|Default|GetCoordPlayer2_3) (Math|Rotator|MakeRotator 0.0 _return_value_y__pitch__13 _returnvalue_yaw_13) false false (Variables|Default|GetOver%20Time) false))
    (:then_10
      (Components|MoveComponentTo _player2_4 (Variables|Default|GetCoordPlayer2_4) (Math|Rotator|MakeRotator 0.0 _return_value_y__pitch__14 _returnvalue_yaw_14) false false (Variables|Default|GetOver%20Time) false))
    (:then_11
      (Components|MoveComponentTo _player2_5 (Variables|Default|GetCoordPlayer2_5) (Math|Rotator|MakeRotator 0.0 _return_value_y__pitch_ _returnvalue_yaw) false false (Variables|Default|GetOver%20Time) false))
    (:then_12
      (Components|MoveComponentTo _player2_6 (Variables|Default|GetCoordPlayer2_6) (Math|Rotator|MakeRotator 0.0 _return_value_y__pitch__2 _returnvalue_yaw_2) false false (Variables|Default|GetOver%20Time) false))
    (:then_13
      (Components|MoveComponentTo _player2_7 (Variables|Default|GetCoordPlayer2_7) (Math|Rotator|MakeRotator 0.0 _return_value_y__pitch__10 _returnvalue_yaw_10) false false (Variables|Default|GetOver%20Time) false))))

(event EventBeginPlay
  (bind _returnvalue (Utilities|Time|SetTimerbyEvent (delegate Custom|MoveMark) 0.2 true))
  (Variables|Default|SetMoveTimer _returnvalue)
  (EventDispatchers|BindEventtoWebSocketonConnectedDelegate (EventDispatchers|CreateEvent :!event Custom|WebSocketConected))
  (EventDispatchers|BindEventtoWebSocketonConnectionErrorDelegate (EventDispatchers|CreateEvent :!event Custom|WebSocketConectedError))
  (EventDispatchers|BindEventtoWebSocketonClosedDelegate (EventDispatchers|CreateEvent :!event Custom|WebSocketClosed))
  (EventDispatchers|BindEventtoWebSocketonMessageDelegate (EventDispatchers|CreateEvent :!event Custom|WebSocketTextMessage))
  (Class|WebSocketClientActor|StartWebSocketClient "ws://ovr-admin.yourneeds.ru:9091/expo/p3/distribution/timer12sec/1301" "ws"))

(event Collision|EventActorBeginOverlap
  (params (OtherActor :type Actor%20Object%20Reference)))

(event EventTick
  (params (DeltaSeconds :type Float%20%28single-precision%29)))

(fn ConstructionScript)

(fn DebugFunc
  (params (A :type String) (C :type String) (InBool :type Boolean))
  (Development|PrintString (Utilities|String|Append A " " C " " (Utilities|String|ToString(Boolean) InBool)) true true "(R=1.000000,G=1.000000,B=1.000000,A=1.000000)" 0.017))