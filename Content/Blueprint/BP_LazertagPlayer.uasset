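; Laser tag player Blueprint that displays a floating nameplate with team-colored nickname and health.
; Tick turns the PlayerLogo widget toward the camera and scales it by distance within clamped limits.
; HealthUpdate animates health drops through a Timeline, ignoring calls while it plays, and updates CurrentHealth when finished.
; At zero health the widget dissolves with an effect sized to it at BeginPlay; ReInitializeActor deactivates that effect.
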(event Custom|ReInitializeActor
  (Components|Activation|Deactivate (Variables|Default|GetWidgetDissolveEffect)))

(event Custom|HealthUpdate
  (params (NewHealth :type Float%20%28double-precision%29))
  (bind _nicknamewidget (Variables|Default|GetNicknameWidget))
  (if (< NewHealth (Variables|Default|GetCurrentHealth))
    (if (not (Variables|Default|GetIsTimelinePlaying))
      (Variables|Default|SetIsTimelinePlaying true)
      (bind _healthtrack (Timeline|Timeline PlayFromStart)
        (:Update
          (Default|UpdateHealthValue _nicknamewidget (Math|Float|MapRangeClamped (- (Variables|Default|GetCurrentHealth) _healthtrack) 0.0 1e+02 0.0 1.0)))
        (:Finished
          (bind _output_get (Variables|Default|SetCurrentHealth NewHealth))
          (Variables|Default|SetIsTimelinePlaying false)
          (if (not (> _output_get 0.0))
            (Components|Activation|Activate (Variables|Default|GetWidgetDissolveEffect) false)
            (Default|MakeWidgetDissolve _nicknamewidget)))))))

(event EventTick
  (params (DeltaSeconds :type Float%20%28single-precision%29))
  (bind _returnvalue (Game|GetPlayerCameraManager 0))
  (bind _playerlogo (Variables|Default|GetPlayerLogo))
  (bind _returnvalue_2 (Transformation|GetActorLocation _returnvalue))
  (bind _returnvalue_3 (Transformation|GetWorldLocation _playerlogo))
  (bind _returnvalue_4 (- _returnvalue_3 _returnvalue_2))
  (bind _returnvalue_5 (Math|Vector|VectorLength _returnvalue_4))
  (bind _returnvalue_6 (* "1.000000,1.000000,1.000000" _returnvalue_5))
  (bind _returnvalue_7 (/ _returnvalue_6 1200))
  (Utilities|IsValid _returnvalue
    (:Is%20Valid
      (Transformation|SetWorldRotation _playerlogo (Math|Rotator|FindLookatRotation _returnvalue_3 _returnvalue_2) true false)
      (Transformation|SetRelativeScale3D _playerlogo (Math|Vector|MakeVector (Math|Float|Clamp(Float) (.x _returnvalue_7) 0.2 1.2) (Math|Float|Clamp(Float) (.y _returnvalue_7) 0.2 1.2) (Math|Float|Clamp(Float) (.z _returnvalue_7) 0.2 1.2))))))

(event EventBeginPlay
  (bind _playerlogo (Variables|Default|GetPlayerLogo))
  (bind _returnvalue (UserInterface|GetWidget _playerlogo))
  (bind _returnvalue_2 (Class|Widget|GetDesiredSize _returnvalue))
  (bind _aswbp_nickname_v_2 (Utilities|Casting|CastToWBP_Nickname_v2 _returnvalue))
  (bind _output_get (Variables|Default|SetNicknameWidget _aswbp_nickname_v_2))
  (Default|SetNicknameText _output_get (Variables|Default|GetNicknameText) (Variables|Default|GetTeamColor) (Variables|Default|GetNicknameOutlinecolor) (Variables|Default|GetOutlineSize))
  (Utilities|FlowControl|Delay 0.2)
  (Niagara|SetNiagaraVariable(Vector3) (Variables|Default|GetWidgetDissolveEffect) "WidgetSize" (Math|Vector|MakeVector (.x _returnvalue_2) 0.0 (.y _returnvalue_2))))

(fn ConstructionScript)