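; BP_HideWebSoket turns WebSocket match statistics into per-player flags on WebSoketActor, for two teams of up to seven players.
; WSTM stores the latest JSON message, and CustomEvent parses it, flagging players whose status is "playing" and current round is "live".
; The socket connection, delegate bindings and looping timer meant to drive this are unwired from BeginPlay.
; Several unused NewMacro copies of the flag logic remain.
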(event Custom|CustomEvent
  (bind _websoketactor (Variables|Default|GetWebSoketActor))
  (bind _websoketactor_2 (Variables|Default|GetWebSoketActor))
  (Utilities|IsValid (Variables|Default|GetWebSoketActor)
    (:Is%20Valid
      (for (_array_element _array_index) (Class|BlueprintJsonLibrary|ToArray(JsonValue) (Class|BlueprintJsonLibrary|ToJsonValue(JsonObject) (Class|BlueprintJsonLibrary|ToJsonObject(String) (Variables|Default|GetMessage)) "teams"))
        (switch string (Utilities|String|ToString(Integer) _array_index)
          (:0
            (for (_array_element_2 _array_index_2) (Class|BlueprintJsonLibrary|ToArray(JsonValue) (Class|BlueprintJsonLibrary|ToJsonValue(JsonObject) (Class|BlueprintJsonLibrary|ToObject(JsonValue) _array_element) "athletes"))
              (switch string (Utilities|String|ToString(Integer) _array_index_2)
                (:0
                  (Variables|/Game/BP_WebsoketActor.BP_WebsoketActor_C|SetPlaer1_1 _websoketactor (and (Utilities|Enum|Equal(Enum) (Class|BlueprintJsonLibrary|ToString(JsonValue) (Class|BlueprintJsonLibrary|ToJsonValue(JsonObject) (Class|BlueprintJsonLibrary|ToObject(JsonValue) (Class|BlueprintJsonLibrary|ToJsonValue(JsonObject) (Class|BlueprintJsonLibrary|ToObject(JsonValue) _array_element_2) "info")) "status")) "playing") (Utilities|Enum|Equal(Enum) (Class|BlueprintJsonLibrary|ToString(JsonValue) (Class|BlueprintJsonLibrary|ToJsonValue(JsonObject) (Class|BlueprintJsonLibrary|ToObject(JsonValue) (Class|BlueprintJsonLibrary|ToJsonValue(JsonObject) (Class|BlueprintJsonLibrary|ToObject(JsonValue) (Class|BlueprintJsonLibrary|ToJsonValue(JsonObject) (Class|BlueprintJsonLibrary|ToObject(JsonValue) _array_element_2) "statistic")) "currentRound")) "status")) "live"))))
                (:1
                  (Variables|/Game/BP_WebsoketActor.BP_WebsoketActor_C|SetPlaer1_2 _websoketactor (and (Utilities|Enum|Equal(Enum) (Class|BlueprintJsonLibrary|ToString(JsonValue) (Class|BlueprintJsonLibrary|ToJsonValue(JsonObject) (Class|BlueprintJsonLibrary|ToObject(JsonValue) (Class|BlueprintJsonLibrary|ToJsonValue(JsonObject) (Class|BlueprintJsonLibrary|ToObject(JsonValue) _array_element_2) "info")) "status")) "playing") (Utilities|Enum|Equal(Enum) (Class|BlueprintJsonLibrary|ToString(JsonValue) (Class|BlueprintJsonLibrary|ToJsonValue(JsonObject) (Class|BlueprintJsonLibrary|ToObject(JsonValue) (Class|BlueprintJsonLibrary|ToJsonValue(JsonObject) (Class|BlueprintJsonLibrary|ToObject(JsonValue) (Class|BlueprintJsonLibrary|ToJsonValue(JsonObject) (Class|BlueprintJsonLibrary|ToObject(JsonValue) _array_element_2) "statistic")) "currentRound")) "status")) "live"))))
                (:2
                  (Variables|/Game/BP_WebsoketActor.BP_WebsoketActor_C|SetPlaer1_3 _websoketactor (and (Utilities|Enum|Equal(Enum) (Class|BlueprintJsonLibrary|ToString(JsonValue) (Class|BlueprintJsonLibrary|ToJsonValue(JsonObject) (Class|BlueprintJsonLibrary|ToObject(JsonValue) (Class|BlueprintJsonLibrary|ToJsonValue(JsonObject) (Class|BlueprintJsonLibrary|ToObject(JsonValue) _array_element_2) "info")) "status")) "playing") (Utilities|Enum|Equal(Enum) (Class|BlueprintJsonLibrary|ToString(JsonValue) (Class|BlueprintJsonLibrary|ToJsonValue(JsonObject) (Class|BlueprintJsonLibrary|ToObject(JsonValue) (Class|BlueprintJsonLibrary|ToJsonValue(JsonObject) (Class|BlueprintJsonLibrary|ToObject(JsonValue) (Class|BlueprintJsonLibrary|ToJsonValue(JsonObject) (Class|BlueprintJsonLibrary|ToObject(JsonValue) _array_element_2) "statistic")) "currentRound")) "status")) "live"))))
                (:3
                  (Variables|/Game/BP_WebsoketActor.BP_WebsoketActor_C|SetPlaer1_4 _websoketactor (and (Utilities|Enum|Equal(Enum) (Class|BlueprintJsonLibrary|ToString(JsonValue) (Class|BlueprintJsonLibrary|ToJsonValue(JsonObject) (Class|BlueprintJsonLibrary|ToObject(JsonValue) (Class|BlueprintJsonLibrary|ToJsonValue(JsonObject) (Class|BlueprintJsonLibrary|ToObject(JsonValue) _array_element_2) "info")) "status")) "playing") (Utilities|Enum|Equal(Enum) (Class|BlueprintJsonLibrary|ToString(JsonValue) (Class|BlueprintJsonLibrary|ToJsonValue(JsonObject) (Class|BlueprintJsonLibrary|ToObject(JsonValue) (Class|BlueprintJsonLibrary|ToJsonValue(JsonObject) (Class|BlueprintJsonLibrary|ToObject(JsonValue) (Class|BlueprintJsonLibrary|ToJsonValue(JsonObject) (Class|BlueprintJsonLibrary|ToObject(JsonValue) _array_element_2) "statistic")) "currentRound")) "status")) "live"))))
                (:4
                  (Variables|/Game/BP_WebsoketActor.BP_WebsoketActor_C|SetPlaer1_5 _websoketactor (and (Utilities|Enum|Equal(Enum) (Class|BlueprintJsonLibrary|ToString(JsonValue) (Class|BlueprintJsonLibrary|ToJsonValue(JsonObject) (Class|BlueprintJsonLibrary|ToObject(JsonValue) (Class|BlueprintJsonLibrary|ToJsonValue(JsonObject) (Class|BlueprintJsonLibrary|ToObject(JsonValue) _array_element_2) "info")) "status")) "playing") (Utilities|Enum|Equal(Enum) (Class|BlueprintJsonLibrary|ToString(JsonValue) (Class|BlueprintJsonLibrary|ToJsonValue(JsonObject) (Class|BlueprintJsonLibrary|ToObject(JsonValue) (Class|BlueprintJsonLibrary|ToJsonValue(JsonObject) (Class|BlueprintJsonLibrary|ToObject(JsonValue) (Class|BlueprintJsonLibrary|ToJsonValue(JsonObject) (Class|BlueprintJsonLibrary|ToObject(JsonValue) _array_element_2) "statistic")) "currentRound")) "status")) "live"))))
                (:5
                  (Variables|/Game/BP_WebsoketActor.BP_WebsoketActor_C|SetPlaer1_6 _websoketactor (and (Utilities|Enum|Equal(Enum) (Class|BlueprintJsonLibrary|ToString(JsonValue) (Class|BlueprintJsonLibrary|ToJsonValue(JsonObject) (Class|BlueprintJsonLibrary|ToObject(JsonValue) (Class|BlueprintJsonLibrary|ToJsonValue(JsonObject) (Class|BlueprintJsonLibrary|ToObject(JsonValue) _array_element_2) "info")) "status")) "playing") (Utilities|Enum|Equal(Enum) (Class|BlueprintJsonLibrary|ToString(JsonValue) (Class|BlueprintJsonLibrary|ToJsonValue(JsonObject) (Class|BlueprintJsonLibrary|ToObject(JsonValue) (Class|BlueprintJsonLibrary|ToJsonValue(JsonObject) (Class|BlueprintJsonLibrary|ToObject(JsonValue) (Class|BlueprintJsonLibrary|ToJsonValue(JsonObject) (Class|BlueprintJsonLibrary|ToObject(JsonValue) _array_element_2) "statistic")) "currentRound")) "status")) "live"))))
                (:6
                  (Variables|/Game/BP_WebsoketActor.BP_WebsoketActor_C|SetPlaer1_7 _websoketactor (and (Utilities|Enum|Equal(Enum) (Class|BlueprintJsonLibrary|ToString(JsonValue) (Class|BlueprintJsonLibrary|ToJsonValue(JsonObject) (Class|BlueprintJsonLibrary|ToObject(JsonValue) (Class|BlueprintJsonLibrary|ToJsonValue(JsonObject) (Class|BlueprintJsonLibrary|ToObject(JsonValue) _array_element_2) "info")) "status")) "playing") (Utilities|Enum|Equal(Enum) (Class|BlueprintJsonLibrary|ToString(JsonValue) (Class|BlueprintJsonLibrary|ToJsonValue(JsonObject) (Class|BlueprintJsonLibrary|ToObject(JsonValue) (Class|BlueprintJsonLibrary|ToJsonValue(JsonObject) (Class|BlueprintJsonLibrary|ToObject(JsonValue) (Class|BlueprintJsonLibrary|ToJsonValue(JsonObject) (Class|BlueprintJsonLibrary|ToObject(JsonValue) _array_element_2) "statistic")) "currentRound")) "status")) "live")))))))
          (:1
            (for (_array_element_3 _array_index_3) (Class|BlueprintJsonLibrary|ToArray(JsonValue) (Class|BlueprintJsonLibrary|ToJsonValue(JsonObject) (Class|BlueprintJsonLibrary|ToObject(JsonValue) _array_element) "athletes"))
              (switch string (Utilities|String|ToString(Integer) _array_index_3)
                (:0
                  (Variables|/Game/BP_WebsoketActor.BP_WebsoketActor_C|SetPlaer2_1 _websoketactor_2 (and (Utilities|Enum|Equal(Enum) (Class|BlueprintJsonLibrary|ToString(JsonValue) (Class|BlueprintJsonLibrary|ToJsonValue(JsonObject) (Class|BlueprintJsonLibrary|ToObject(JsonValue) (Class|BlueprintJsonLibrary|ToJsonValue(JsonObject) (Class|BlueprintJsonLibrary|ToObject(JsonValue) _array_element_3) "info")) "status")) "playing") (Utilities|Enum|Equal(Enum) (Class|BlueprintJsonLibrary|ToString(JsonValue) (Class|BlueprintJsonLibrary|ToJsonValue(JsonObject) (Class|BlueprintJsonLibrary|ToObject(JsonValue) (Class|BlueprintJsonLibrary|ToJsonValue(JsonObject) (Class|BlueprintJsonLibrary|ToObject(JsonValue) (Class|BlueprintJsonLibrary|ToJsonValue(JsonObject) (Class|BlueprintJsonLibrary|ToObject(JsonValue) _array_element_3) "statistic")) "currentRound")) "status")) "live"))))
                (:1
                  (Variables|/Game/BP_WebsoketActor.BP_WebsoketActor_C|SetPlaer2_2 _websoketactor_2 (and (Utilities|Enum|Equal(Enum) (Class|BlueprintJsonLibrary|ToString(JsonValue) (Class|BlueprintJsonLibrary|ToJsonValue(JsonObject) (Class|BlueprintJsonLibrary|ToObject(JsonValue) (Class|BlueprintJsonLibrary|ToJsonValue(JsonObject) (Class|BlueprintJsonLibrary|ToObject(JsonValue) _array_element_3) "info")) "status")) "playing") (Utilities|Enum|Equal(Enum) (Class|BlueprintJsonLibrary|ToString(JsonValue) (Class|BlueprintJsonLibrary|ToJsonValue(JsonObject) (Class|BlueprintJsonLibrary|ToObject(JsonValue) (Class|BlueprintJsonLibrary|ToJsonValue(JsonObject) (Class|BlueprintJsonLibrary|ToObject(JsonValue) (Class|BlueprintJsonLibrary|ToJsonValue(JsonObject) (Class|BlueprintJsonLibrary|ToObject(JsonValue) _array_element_3) "statistic")) "currentRound")) "status")) "live"))))
                (:2
                  (Variables|/Game/BP_WebsoketActor.BP_WebsoketActor_C|SetPlaer2_3 _websoketactor_2 (and (Utilities|Enum|Equal(Enum) (Class|BlueprintJsonLibrary|ToString(JsonValue) (Class|BlueprintJsonLibrary|ToJsonValue(JsonObject) (Class|BlueprintJsonLibrary|ToObject(JsonValue) (Class|BlueprintJsonLibrary|ToJsonValue(JsonObject) (Class|BlueprintJsonLibrary|ToObject(JsonValue) _array_element_3) "info")) "status")) "playing") (Utilities|Enum|Equal(Enum) (Class|BlueprintJsonLibrary|ToString(JsonValue) (Class|BlueprintJsonLibrary|ToJsonValue(JsonObject) (Class|BlueprintJsonLibrary|ToObject(JsonValue) (Class|BlueprintJsonLibrary|ToJsonValue(JsonObject) (Class|BlueprintJsonLibrary|ToObject(JsonValue) (Class|BlueprintJsonLibrary|ToJsonValue(JsonObject) (Class|BlueprintJsonLibrary|ToObject(JsonValue) _array_element_3) "statistic")) "currentRound")) "status")) "live"))))
                (:3
                  (Variables|/Game/BP_WebsoketActor.BP_WebsoketActor_C|SetPlaer2_4 _websoketactor_2 (and (Utilities|Enum|Equal(Enum) (Class|BlueprintJsonLibrary|ToString(JsonValue) (Class|BlueprintJsonLibrary|ToJsonValue(JsonObject) (Class|BlueprintJsonLibrary|ToObject(JsonValue) (Class|BlueprintJsonLibrary|ToJsonValue(JsonObject) (Class|BlueprintJsonLibrary|ToObject(JsonValue) _array_element_3) "info")) "status")) "playing") (Utilities|Enum|Equal(Enum) (Class|BlueprintJsonLibrary|ToString(JsonValue) (Class|BlueprintJsonLibrary|ToJsonValue(JsonObject) (Class|BlueprintJsonLibrary|ToObject(JsonValue) (Class|BlueprintJsonLibrary|ToJsonValue(JsonObject) (Class|BlueprintJsonLibrary|ToObject(JsonValue) (Class|BlueprintJsonLibrary|ToJsonValue(JsonObject) (Class|BlueprintJsonLibrary|ToObject(JsonValue) _array_element_3) "statistic")) "currentRound")) "status")) "live"))))
                (:4
                  (Variables|/Game/BP_WebsoketActor.BP_WebsoketActor_C|SetPlaer2_5 _websoketactor_2 (and (Utilities|Enum|Equal(Enum) (Class|BlueprintJsonLibrary|ToString(JsonValue) (Class|BlueprintJsonLibrary|ToJsonValue(JsonObject) (Class|BlueprintJsonLibrary|ToObject(JsonValue) (Class|BlueprintJsonLibrary|ToJsonValue(JsonObject) (Class|BlueprintJsonLibrary|ToObject(JsonValue) _array_element_3) "info")) "status")) "playing") (Utilities|Enum|Equal(Enum) (Class|BlueprintJsonLibrary|ToString(JsonValue) (Class|BlueprintJsonLibrary|ToJsonValue(JsonObject) (Class|BlueprintJsonLibrary|ToObject(JsonValue) (Class|BlueprintJsonLibrary|ToJsonValue(JsonObject) (Class|BlueprintJsonLibrary|ToObject(JsonValue) (Class|BlueprintJsonLibrary|ToJsonValue(JsonObject) (Class|BlueprintJsonLibrary|ToObject(JsonValue) _array_element_3) "statistic")) "currentRound")) "status")) "live"))))
                (:5
                  (Variables|/Game/BP_WebsoketActor.BP_WebsoketActor_C|SetPlaer2_6 _websoketactor_2 (and (Utilities|Enum|Equal(Enum) (Class|BlueprintJsonLibrary|ToString(JsonValue) (Class|BlueprintJsonLibrary|ToJsonValue(JsonObject) (Class|BlueprintJsonLibrary|ToObject(JsonValue) (Class|BlueprintJsonLibrary|ToJsonValue(JsonObject) (Class|BlueprintJsonLibrary|ToObject(JsonValue) _array_element_3) "info")) "status")) "playing") (Utilities|Enum|Equal(Enum) (Class|BlueprintJsonLibrary|ToString(JsonValue) (Class|BlueprintJsonLibrary|ToJsonValue(JsonObject) (Class|BlueprintJsonLibrary|ToObject(JsonValue) (Class|BlueprintJsonLibrary|ToJsonValue(JsonObject) (Class|BlueprintJsonLibrary|ToObject(JsonValue) (Class|BlueprintJsonLibrary|ToJsonValue(JsonObject) (Class|BlueprintJsonLibrary|ToObject(JsonValue) _array_element_3) "statistic")) "currentRound")) "status")) "live"))))
                (:6
                  (Variables|/Game/BP_WebsoketActor.BP_WebsoketActor_C|SetPlaer2_7 _websoketactor_2 (and (Utilities|Enum|Equal(Enum) (Class|BlueprintJsonLibrary|ToString(JsonValue) (Class|BlueprintJsonLibrary|ToJsonValue(JsonObject) (Class|BlueprintJsonLibrary|ToObject(JsonValue) (Class|BlueprintJsonLibrary|ToJsonValue(JsonObject) (Class|BlueprintJsonLibrary|ToObject(JsonValue) _array_element_3) "info")) "status")) "playing") (Utilities|Enum|Equal(Enum) (Class|BlueprintJsonLibrary|ToString(JsonValue) (Class|BlueprintJsonLibrary|ToJsonValue(JsonObject) (Class|BlueprintJsonLibrary|ToObject(JsonValue) (Class|BlueprintJsonLibrary|ToJsonValue(JsonObject) (Class|BlueprintJsonLibrary|ToObject(JsonValue) (Class|BlueprintJsonLibrary|ToJsonValue(JsonObject) (Class|BlueprintJsonLibrary|ToObject(JsonValue) _array_element_3) "statistic")) "currentRound")) "status")) "live"))))))))))))

(event Custom|WSC
  (params (b :type Boolean))
  (Development|PrintString (Utilities|String|Append "Conected: " (Utilities|String|ToString(Boolean) b)) true true "(R=0.449535,G=0.956847,B=1.000000,A=1.000000)" 2e+01))

(event Custom|WSCE
  (params (error :type String))
  (Development|PrintString (Utilities|String|Append "Conected Error: " error) true true "(R=1.000000,G=0.000000,B=0.064424,A=1.000000)" 2e+01))

(event Custom|WSCL
  (params (StatusCode :type Integer) (Reason :type String) (bWasClean :type Boolean))
  (Development|PrintString (Utilities|String|Append "Conected close: " (Utilities|String|ToString(Integer) StatusCode)) true true "(R=0.000000,G=1.000000,B=0.974743,A=1.000000)" 3e+02)
  (Utilities|Time|ClearandInvalidateTimerbyHandle (Variables|Default|GetNewVar)))

(event Custom|WSTM
  (params (message :type String))
  (Variables|Default|SetMessage message))

(event Custom|WSRM
  (params (data :type Array%20of%20Bytes) (Size :type Integer) (BytesRemaining :type Integer)))

(event EventBeginPlay)

(event Collision|EventActorBeginOverlap
  (params (OtherActor :type Actor%20Object%20Reference)))

(event EventTick
  (params (DeltaSeconds :type Float%20%28single-precision%29)))

(fn ConstructionScript)